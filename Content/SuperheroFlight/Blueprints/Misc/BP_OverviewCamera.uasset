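; BP_OverviewCamera plays an optional intro camera sequence that tours the level before handing the view back to the player.
; On BeginPlay, after a start delay, it walks an array of cameras, pausing on each for a set time.
; It cuts instantly to the first camera, blends cubically to the rest, then blends to the player character once the array runs out.
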(event `self.ReceiveBeginPlay`
  (bind _output (`|GetArrayItem` (`self.Camera`) (`self.CameraIndex`)))
  (if (`self.UseCamera`)
    (`KismetSystemLibrary.Delay` (`self.StartDelay`))
    (`/Engine/EditorBlueprintResources/StandardMacros.IsValid` _output :!label _label
      (:`Is Valid`
        (`PlayerController.SetViewTargetWithBlend` (`GameplayStatics.GetPlayerController` 0) _output (select `bool` (== (`self.CameraIndex`) 0) :`false` 2.0) "VTBlend_Cubic" 2.0 false)
        (`KismetSystemLibrary.Delay` (`self.Delay`))
        (`/Engine/EditorBlueprintResources/StandardMacros.IncrementInt` (`self.CameraIndex`)
          (:`  `
            (goto _label))))
      (:`Is Not Valid`
        (`PlayerController.SetViewTargetWithBlend` (`GameplayStatics.GetPlayerController` 0) (`GameplayStatics.GetPlayerCharacter` 0) 2.0 "VTBlend_Cubic" 2.0 false)))))

(fn `UserConstructionScript`)